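; Player character Blueprint that handles pause menu toggling and a "Time Pause" effect on input.
; PauseGame pauses the game and shows the PauseMenu widget with a cursor; UnPauseGame clears all widgets, restores game-only input and creates a fresh HUD.
; Time Pause flip-flops post-process weight, background music and stop/resume/tick sounds, without changing game time here.
; RetryGame is an empty stub.
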(event `InputAction|PauseGame` :consume false
  (params (Key :type "Key Structure"))
  (:`Pressed`
    (if (`self.Game Paused?`)
      (`self.UnPauseGame`)
      (else
        (`self.PauseGame`)))))

(event `InputAction|Time Pause` :consume false
  (params (Key :type "Key Structure"))
  (bind _postprocess (`self.PostProcess`))
  (bind _timestop (`self.TimeStop`))
  (bind _timeresume (`self.TimeResume`))
  (bind _timestoptick (`self.TimeStopTick`))
  (bind _backgroundmusic (`self.BackgroundMusic`))
  (:`Pressed`
    (`/Engine/EditorBlueprintResources/StandardMacros.FlipFlop`
      (:`A`
        (set `PostProcessComponent.BlendWeight` 1.0 _postprocess)
        (`AudioComponent.SetPaused` _backgroundmusic true)
        (`AudioComponent.Stop` _timeresume)
        (`AudioComponent.Play` _timestop 0.0)
        (`AudioComponent.Play` _timestoptick 0.0))
      (:`B`
        (set `PostProcessComponent.BlendWeight` 0.0 _postprocess)
        (`AudioComponent.SetPaused` _backgroundmusic false)
        (`AudioComponent.Stop` _timestop)
        (`AudioComponent.Play` _timeresume 0.0)
        (`AudioComponent.Stop` _timestoptick)))))

(fn `PauseGame`
  (bind _returnvalue (`GameplayStatics.GetPlayerController` 0))
  (set `self.Game Paused?` true)
  (`GameplayStatics.SetGamePaused` true)
  (bind _returnvalue_2 (`|CreateWidget` "/Game/Blueprints/PauseMenu.PauseMenu_C" _returnvalue))
  (bind _output_get (set `self.Pause Menu` _returnvalue_2))
  (`UserWidget.AddToViewport` _output_get 0)
  (`WidgetBlueprintLibrary.SetInputMode_GameAndUIEx` _returnvalue (`self.Pause Menu`) "DoNotLock" false)
  (set `PlayerController.bShowMouseCursor` true _returnvalue))

(fn `RetryGame`)

(fn `UnPauseGame`
  (bind _returnvalue (`GameplayStatics.GetPlayerController` 0))
  (set `self.Game Paused?` false)
  (`GameplayStatics.SetGamePaused` false)
  (`WidgetLayoutLibrary.RemoveAllWidgets`)
  (`WidgetBlueprintLibrary.SetInputMode_GameOnly` _returnvalue)
  (set `PlayerController.bShowMouseCursor` false _returnvalue)
  (bind _returnvalue_2 (`|CreateWidget` "/Game/Blueprints/HUD.HUD_C" _returnvalue))
  (`UserWidget.AddToViewport` _returnvalue_2 0))

(fn `UserConstructionScript`)